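; Player character with a toggled top-down aim mode for marking and "shooting" targets, plus a dolly zoom camera effect.
; E freezes movement and swings the camera boom by timeline, showing a cursor decal; left click records actors and stamps hit decals.
; When the reverse finishes, movement resumes and one undelayed loop faces each target, plays a shot sound and prints its name.
; P toggles the dolly zoom, lerping FOV against arm length.
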(event `Key|E`
  (params (Key :type "Key Structure" :default "AnyKey"))
  ;[1 1 1] TopDown Aim
  (:`Pressed`
    (`self.SetMovementActive` false)
    (`/Engine/EditorBlueprintResources/StandardMacros.FlipFlop`
      (:`A`
        (bind (_direction _cameraupdown) (`Timeline|TopDownAimTimelIne` :!label _label)
          (:`Update`
            (`self.TopDownRotation` _cameraupdown))
          (:`Finished`
            (switch `ETimelineDirection` _direction
              (:`Forward`
                (`self.SetMovementActive` false)
                (`SceneComponent.SetVisibility` (`self.MousePositionDecal`) true false))
              (:`Backward`
                (`self.SetMovementActive` true)
                (`SceneComponent.SetVisibility` (`self.MousePositionDecal`) false false)
                (`self.ShootHitActors`))))))
      (:`B`
        (`SceneComponent.SetVisibility` (`self.MousePositionDecal`) false false)
        (goto _label :!via `Reverse`)))))

(event `Key|P`
  (params (Key :type "Key Structure" :default "AnyKey"))
  ;[1 1 1] DollyZoom
  (:`Pressed`
    (`/Engine/EditorBlueprintResources/StandardMacros.FlipFlop`
      (:`A`
        (bind (_direction _zoom_fov_stuff) (`Timeline|DollyZoomTimeline` :!label _label_2)
          (:`Update`
            (`self.DollyZoom` _zoom_fov_stuff))))
      (:`B`
        (goto _label_2 :!via `Reverse`)))))

(event `self.ReceiveTick`
  (params (DeltaSeconds :type "Float (single-precision)"))
  (if (`SceneComponent.IsVisible` (`self.MousePositionDecal`))
    (`self.SetMouseDecalPos`)))

(event `Key|LeftMouseButton`
  (params (Key :type "Key Structure" :default "AnyKey"))
  (:`Pressed`
    (if (`SceneComponent.IsVisible` (`self.MousePositionDecal`))
      (bind (_hitactor _hitcomponent _hittransform) (`self.GetActorUnderMouse`))
      (`/Engine/EditorBlueprintResources/StandardMacros.IsValid` _hitactor
        (:`Is Valid`
          (`GameplayStatics.SpawnDecalAttached` "/Game/LowPoly/Stuey/Materials/M_Decal_Hit.M_Decal_Hit" (16.0 32.0 32.0) _hitcomponent "None" (.location _hittransform) (.rotation _hittransform) "KeepWorldPosition"))))))

(fn `DollyZoom`
  (params (FOVAlpha :type "Float (double-precision)"))
  (locals (FOVShort :type "Float (double-precision)" :default 90.0) (FOVLong :type "Float (double-precision)" :default 135.0) (ArmShort :type "Float (double-precision)" :default 430.0) (ArmLong :type "Float (double-precision)" :default 900.0))
  (`CameraComponent.SetFieldOfView` (`self.FollowCamera`) (`KismetMathLibrary.Lerp` (`local.FOVShort`) (`local.FOVLong`) FOVAlpha))
  (set `SpringArmComponent.TargetArmLength` (`KismetMathLibrary.Lerp` (`local.ArmLong`) (`local.ArmShort`) FOVAlpha) (`self.CameraBoom`)))

(fn `GetActorUnderMouse`
  (returns (HitActor :type "Actor Object Reference") (HitComponent :type "PrimitiveComponent Object Reference") (HitTransform :type "Transform Structure"))
  (bind (_bblockinghit _binitialoverlap _time _location _impactpoint _normal _impactnormal _physmat _hitactor _hitcomponent) (`GameplayStatics.BreakHitResult` (`PlayerController.GetHitResultUnderCursorForObjects` (`GameplayStatics.GetPlayerController` 0) (`|MakeArray` "ObjectTypeQuery7" :!type "EObjectTypeQuery Enum") true)))
  (`KismetArrayLibrary.Array_Add` (`self.HitActors`) _hitactor)
  (return _hitactor _hitcomponent (`KismetMathLibrary.MakeTransform` _location (`KismetMathLibrary.MakeRotationFromAxes` _impactnormal _impactnormal _impactnormal))))

(fn `SetMouseDecalPos`
  (bind (_bblockinghit _binitialoverlap _time _location _impactpoint _normal _impactnormal) (`GameplayStatics.BreakHitResult` (`PlayerController.GetHitResultUnderCursorByChannel` (`GameplayStatics.GetPlayerController` 0) "TraceTypeQuery1" true)))
  (`SceneComponent.K2_SetWorldLocationAndRotation` (`self.MousePositionDecal`) _location (`KismetMathLibrary.MakeRotationFromAxes` _impactnormal _impactnormal _impactnormal) false false))

(fn `SetMovementActive`
  (params (Active :type Boolean))
  (bind _charactermovement (`self.CharacterMovement`))
  (if (not Active)
    (`MovementComponent.StopMovementImmediately` _charactermovement))
  (`ActorComponent.SetActive` _charactermovement Active false))

(fn `ShootHitActors`
  (bind _returnvalue (`GameplayStatics.GetPlayerPawn` 0))
  (bind _returnvalue_2 (`self.K2_GetActorLocation` _returnvalue))
  (for _array_element (`self.HitActors`)
    (`/Engine/EditorBlueprintResources/StandardMacros.IsValid` _array_element
      (:`Is Valid`
        (`KismetSystemLibrary.PrintString` (`KismetSystemLibrary.GetDisplayName` _array_element))
        (bind (_returnvalue_roll _returnvalue_pitch _returnvalue_yaw) (`KismetMathLibrary.BreakRotator` (`KismetMathLibrary.FindLookAtRotation` _returnvalue_2 (`self.K2_GetActorLocation` _array_element))))
        (`self.K2_SetActorRotation` _returnvalue (`KismetMathLibrary.MakeRotator` 0.0 0.0 _returnvalue_yaw) false)
        (`GameplayStatics.PlaySoundAtLocation` "/Game/SFX/Shoot.Shoot" _returnvalue_2))))
  (`KismetArrayLibrary.Array_Clear` (`self.HitActors`)))

(fn `TopDownRotation`
  (params (RotationAlpha :type "Float (double-precision)"))
  (locals (EndRotation :type "Rotator Structure" :default (struct :`Pitch` -90.0)) (StartRotation :type "Rotator Structure" :default (struct :`Pitch` -30.0)))
  (`SceneComponent.K2_SetRelativeRotation` (`self.CameraBoom`) (`KismetMathLibrary.RLerp` (`local.StartRotation`) (`local.EndRotation`) RotationAlpha) false false))

(fn `UserConstructionScript`)