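; AreaNamer is a trigger actor that marks a named area of the world with its own music.
; When the player pawn begins overlapping it, it writes its AreaName to GameInstance_BP.
; It then finds the first AudioManager in the level and changes the track to its AreaMusic at its MusicVolume, with a short fade-in.
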(event `self.ReceiveActorBeginOverlap`
  (params (OtherActor :type "Actor Object Reference"))
  (if (== OtherActor (`GameplayStatics.GetPlayerPawn` 0))
    (bind _asgame_instance_bp (cast `/Game/Blueprints/Game/GameInstance_BP` (`GameplayStatics.GetGameInstance`)))
    (set `/Game/Blueprints/Game/GameInstance_BP.AreaName` (`self.AreaName`) _asgame_instance_bp)
    (bind _outactors (`GameplayStatics.GetAllActorsOfClass` "/Game/Blueprints/Game/AudioManager.AudioManager_C"))
    (`/Game/Blueprints/Game/AudioManager.ChangeTrack` (`KismetArrayLibrary.Array_Get` _outactors) (`self.AreaMusic`) 1.5 (`self.MusicVolume`))))

(fn `UserConstructionScript`)