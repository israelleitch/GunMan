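; AudioManager is a Blueprint that plays music and crossfades between tracks.
; It alternates between two audio components, Track01 and Track02, with StartMusic playing the first sound on Track01.
; ChangeTrack checks whether Track02 is playing, fades the new sound in on the other component and fades the current one out over the same given time.
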(event `StartMusic`
  (params (StartTrack :type "SoundBase Object Reference"))
  (bind _track01 (`self.Track01`))
  (`AudioComponent.SetSound` _track01 StartTrack)
  (`AudioComponent.Play` _track01 0.0))

(event `ChangeTrack`
  (params (NewTrack :type "SoundBase Object Reference") (FadeInTime :type "Float (double-precision)"))
  (bind _track01 (`self.Track01`))
  (bind _track02 (`self.Track02`))
  (if (`AudioComponent.IsPlaying` (`self.Track02`))
    (`AudioComponent.SetSound` _track01 NewTrack)
    (`AudioComponent.FadeIn` _track01 FadeInTime 1.0 0.0)
    (`AudioComponent.FadeOut` (`self.Track02`) FadeInTime 0.0)
    (else
      (`AudioComponent.SetSound` _track02 NewTrack)
      (`AudioComponent.FadeIn` _track02 FadeInTime 1.0 0.0)
      (`AudioComponent.FadeOut` (`self.Track01`) FadeInTime 0.0))))

(fn `UserConstructionScript`)