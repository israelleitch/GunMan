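; HUD Blueprint that creates and adds the game's top-level widgets to the viewport for the owning player controller.
; InitialiseHUD branches on IsMenuMap: menu maps get the main menu and quit menu.
; Other maps get a loading screen, started immediately through its Loading call, then the main HUD and quit menu.
; Each widget reference is stored in a variable.
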(event `InitialiseHUD`
  (if (`self.IsMenuMap`)
    (`|ExecutionSequence`
      (:`then_0`
        ;[1 1 1] MainMenu
        (bind _returnvalue (`|CreateWidget` "/Game/Blueprints/UI/Menus/MainMenuWidget.MainMenuWidget_C" (`self.MyPC`)))
        (bind _output_get (set `self.MainMenuWidget` _returnvalue))
        (`UserWidget.AddToViewport` _output_get 0))
      (:`then_1`
        ;[1 1 1] QuitMenu
        (bind _returnvalue_2 (`|CreateWidget` "/Game/Blueprints/UI/Menus/QuitWidget.QuitWidget_C" (`self.MyPC`)))
        (bind _output_get_2 (set `self.QuitWidget` _returnvalue_2))
        (`UserWidget.AddToViewport` _output_get_2 0)))
    (else
      (`|ExecutionSequence`
        (:`then_0`
          ;[1 1 1] LoadingScreen
          (bind _returnvalue_3 (`|CreateWidget` "/Game/Blueprints/UI/Menus/LoadingWidget.LoadingWidget_C" (`self.MyPC`)))
          (bind _output_get_3 (set `self.LoadingWidget` _returnvalue_3))
          (`UserWidget.AddToViewport` _output_get_3 0)
          (`/Game/Blueprints/UI/Menus/LoadingWidget.Loading` _output_get_3))
        (:`then_1`
          ;[1 1 1] MainHUD
          (bind _returnvalue_4 (`|CreateWidget` "/Game/Blueprints/UI/MainHUD/HUD_Master.HUD_Master_C" (`self.MyPC`)))
          (bind _output_get_4 (set `self.HUD_Main` _returnvalue_4))
          (`UserWidget.AddToViewport` _output_get_4 0))
        (:`then_2`
          ;[1 1 1] Quit Menu
          (bind _returnvalue_5 (`|CreateWidget` "/Game/Blueprints/UI/Menus/QuitWidget.QuitWidget_C" (`self.MyPC`)))
          (bind _output_get_5 (set `self.QuitWidget` _returnvalue_5))
          (`UserWidget.AddToViewport` _output_get_5 0))))))

(fn `UserConstructionScript`)