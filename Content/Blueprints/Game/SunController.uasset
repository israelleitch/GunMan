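; Sun controller actor that drives a day-night cycle by rotating a directional light and refreshing the sky sphere.
; BeginPlay derives the length of an hour in seconds from DayLengthInMinutes.
; Tick advances and wraps a 24-hour clock, converts it to sun pitch and updates the sky.
; A range check picks full or quarter speed, but shows no input value, so the slower night rate appears to always apply.
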(event `self.ReceiveBeginPlay`
  (bind _output_get (set `self.OneDay` (* (`self.DayLengthInMinutes`) 60.0)))
  (set `self.OneHour` (/ _output_get 24.0)))

(event `self.ReceiveTick`
  (params (DeltaSeconds :type "Float (single-precision)"))
  (bind _hour (`self.Hour`))
  (if (`KismetMathLibrary.InRange_FloatFloat` 0.0 20.0 24.0)
    ;[1 1 1] Day
    (set `self.Hour` (+ _hour (/ DeltaSeconds (`self.OneHour`))))
    (else
      ;[1 1 1] Night - Slower than Day
      (set `self.Hour` (+ (`self.Hour`) (/ (/ DeltaSeconds 4.0) (`self.OneHour`))))))
  (if (or (> _hour 24.0) (< _hour 0.0))
    (bind _output_get (set `self.Hour` 0.0)))
  (bind _output_get_2 (set `self.SunRotation` (+ (* (/ _output_get 4.0) 90.0) 90.0)))
  (`self.K2_SetActorRotation` (`self.DirectionalLight`) (`KismetMathLibrary.MakeRotator` 0.0 _output_get_2) false)
  (`/Game/Blueprints/Misc/BP_Sky_Sphere_menu.UpdateSunDirection` (`self.SkySphere`)))

(fn `UserConstructionScript`)