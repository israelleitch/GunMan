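; CameraRotator is a trigger actor that changes the player's camera angle while StueyCharacter overlaps it.
; On entry it stores the current CameraBoom rotation and passes NewRotation to OnRotateBoxEnter, or prints a warning if they match.
; On exit it passes the stored rotation to OnRotateBoxExit.
; Construction-script logic for center, left and right preset angles is disconnected and never runs.
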(event `self.ReceiveActorBeginOverlap`
  (params (OtherActor :type "Actor Object Reference"))
  (bind _returnvalue (`GameplayStatics.GetPlayerPawn` 0))
  (if (== OtherActor _returnvalue)
    (bind _asstuey_character (cast `/Game/Blueprints/Character/StueyCharacter` _returnvalue))
    (bind _relativerotation (`SceneComponent.RelativeRotation` (`GunfighterCharacter.CameraBoom` _asstuey_character)))
    (if (!= _relativerotation (`self.NewRotation`) :`ErrorTolerance` 0.0)
      (set `self.PreviousRotation` _relativerotation)
      (`/Game/Blueprints/Character/StueyCharacter.OnRotateBoxEnter` _asstuey_character (`self.NewRotation`))
      (else
        (`KismetSystemLibrary.PrintString` "NEW ROTATION AND PREVIOUS ROTATION ARE THE SAME!")))))

(event `self.ReceiveActorEndOverlap`
  (params (OtherActor :type "Actor Object Reference"))
  (bind _returnvalue (`GameplayStatics.GetPlayerPawn` 0))
  (if (== OtherActor _returnvalue)
    (bind _asstuey_character (cast `/Game/Blueprints/Character/StueyCharacter` _returnvalue))
    (`/Game/Blueprints/Character/StueyCharacter.OnRotateBoxExit` _asstuey_character (`self.PreviousRotation`))))

(fn `UserConstructionScript`)