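; Breakable prop, such as a barrel, built on a DestructibleComponent, that drops a potion pickup when broken.
; BreakMe damages the component with an impulse, spawns PotionPickup_BP at the actor's location, then switches the collision object type to Vehicle.
; An unconnected graph holds an opacity fade using translucent oak or pine materials, dynamic instances and a timeline; SetMats is empty, so it never runs.
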(event `SetMats`
  ;[1 1 1] Dodgy Material Opacity Stuff
)

(event `BreakMe`
  (bind _returnvalue (`self.K2_GetActorLocation`))
  ;[1 1 1] break the thing
  (`DestructibleComponent.ApplyDamage` (`self.DestructibleComponent`) 10.0 _returnvalue _returnvalue 2000.0)
  (`|SpawnActorFromClass` "/Game/Blueprints/Items/PotionPickup_BP.PotionPickup_BP_C" (`KismetMathLibrary.Conv_VectorToTransform` _returnvalue) "Undefined" "OverrideRootScale")
  (`PrimitiveComponent.SetCollisionObjectType` (`self.DestructibleComponent`) "ECC_Vehicle"))

(fn `UserConstructionScript`)