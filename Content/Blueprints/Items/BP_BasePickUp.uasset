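; Base pickup actor that the player collects by overlapping it.
; The construction script applies the MyMesh variable to its static mesh component.
; BeginPlay caches the player pawn in MyPawn, and an overlap with that player's pawn calls OnPickup, which only destroys the actor in this base version.
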(event `self.ReceiveBeginPlay`
  (set `self.MyPawn` (`GameplayStatics.GetPlayerPawn` 0)))

(event `self.ReceiveActorBeginOverlap`
  (params (OtherActor :type "Actor Object Reference"))
  (if (== OtherActor (`GameplayStatics.GetPlayerPawn` 0))
    (`self.OnPickup`)))

(fn `OnPickup`
  (`self.K2_DestroyActor`))

(fn `UserConstructionScript`
  (`StaticMeshComponent.SetStaticMesh` (`self.StaticMesh`) (`self.MyMesh`)))