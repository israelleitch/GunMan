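; AI bot character that wanders between random AIStops actors in the level, halting while the player is aiming.
; Construction sets walk speed and picks a random first stop; BeginPlay caches all stops and the StueyCharacter player.
; Tick stops movement but keeps pathing during aiming, otherwise calls SimpleMoveToActor toward the current stop.
; Near the goal, it waits briefly before picking another random stop, possibly the same one.
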(event `self.ReceiveBeginPlay`
  (bind _outactors (`GameplayStatics.GetAllActorsOfClass` "/Game/Blueprints/AI/AIStops.AIStops_C"))
  (set `self.Waypoints` _outactors)
  (bind _asstuey_character (cast `/Game/Blueprints/Character/StueyCharacter` (`GameplayStatics.GetPlayerPawn` 0)))
  (set `self.Player` _asstuey_character))

(event `self.ReceiveTick`
  (params (DeltaSeconds :type "Float (single-precision)"))
  (if (`/Game/Blueprints/Character/StueyCharacter.IsAiming` (`self.Player`))
    (`NavMovementComponent.StopMovementKeepPathing` (`self.CharacterMovement`))
    (else
      (bind _thereyet (`self.CheckIfAtGoal`))
      (if _thereyet
        (`KismetSystemLibrary.Delay` 3.0)
        (`self.GoToNext`)
        (else
          (`self.MoveToGoal`))))))

(fn `CheckIfAtGoal`
  (returns (ThereYet :type Boolean))
  (bind _output_get (set `self.AtGoal` (== (`SceneComponent.K2_GetComponentLocation` (`self.CapsuleComponent`)) (`self.K2_GetActorLocation` (`self.StartingNode`)) :`ErrorTolerance` 100.0)))
  (return _output_get))

(fn `GetRandomWaypoint`
  (bind _outactors (`GameplayStatics.GetAllActorsOfClass` "/Game/Blueprints/AI/AIStops.AIStops_C"))
  (set `self.StartingNode` (`KismetArrayLibrary.Array_Get` _outactors (`KismetMathLibrary.RandomIntegerInRange` 0 (- (`KismetArrayLibrary.Array_Length` _outactors) 1)))))

(fn `GoToNext`
  (bind _waypoints (`self.Waypoints`))
  (set `self.StartingNode` (`KismetArrayLibrary.Array_Get` _waypoints (`KismetMathLibrary.RandomIntegerInRange` 0 (- (`KismetArrayLibrary.Array_Length` _waypoints) 1)))))

(fn `MoveToGoal`
  (`NavigationSystem.SimpleMoveToActor` (`self.GetController`) (`self.StartingNode`)))

(fn `UserConstructionScript`
  (set `CharacterMovementComponent.MaxWalkSpeed` (`self.MyWalkSpeed`) (`self.CharacterMovement`))
  (`self.GetRandomWaypoint`))