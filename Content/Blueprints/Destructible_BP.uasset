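; Breakable wooden prop, such as a barrel, that shatters on BreakMe, spawns a Potion and fades out.
; BreakMe applies damage with an impulse to the destructible component, switches its collision object type to Vehicle, then calls SetMats.
; SetMats swaps every slot to a translucent oak (barrel mesh) or pine material, then creates dynamic instances whose Opacity a timeline drives toward zero.
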(event `SetMats`
  (bind _destructiblecomponent (`self.DestructibleComponent`))
  ;[1 1 1] Dodgy Material Opacity Stuff
  (bind _output_get (set `self.Materials` (`MeshComponent.GetMaterials` (`self.DestructibleComponent`))))
  (for (_ _array_index) _output_get
    (bind _returnvalue (`DestructibleComponent.GetDestructibleMesh` (`self.DestructibleComponent`)))
    (if (== _returnvalue "/Game/Environment/Destructible/BarrelMat_DM.BarrelMat_DM")
      (`PrimitiveComponent.SetMaterial` _destructiblecomponent _array_index "/Game/Blueprints/Materials/M_Wood_Oak_Trans_Inst.M_Wood_Oak_Trans_Inst")
      (else
        (`PrimitiveComponent.SetMaterial` _destructiblecomponent _array_index "/Game/Blueprints/Materials/M_Wood_Pine_trans_Inst.M_Wood_Pine_trans_Inst")))
    (`KismetArrayLibrary.Array_Clear` (`self.Materials`))
    (set `self.Materials` (`MeshComponent.GetMaterials` _destructiblecomponent)))
  (for (_array_element _array_index_2) (`self.Materials`)
    (bind _returnvalue_2 (`PrimitiveComponent.CreateDynamicMaterialInstance` (`self.DestructibleComponent`) _array_index_2 _array_element))
    (bind (_direction _opacity) (`Timeline|OpacityTimeline` :!via `PlayFromStart`)
      (:`Update`
        (`MaterialInstanceDynamic.SetScalarParameterValue` _returnvalue_2 "Opacity" (`KismetMathLibrary.Lerp` 1.0 0.0 _opacity))))))

(event `BreakMe`
  (bind _returnvalue (`self.K2_GetActorLocation`))
  ;[1 1 1] break the thing
  (`DestructibleComponent.ApplyDamage` (`self.DestructibleComponent`) 10.0 _returnvalue _returnvalue 2000.0)
  (`|SpawnActorFromClass` "/Game/Blueprints/Potion.Potion_C" (`KismetMathLibrary.Conv_VectorToTransform` _returnvalue) "Undefined" "OverrideRootScale")
  (`PrimitiveComponent.SetCollisionObjectType` (`self.DestructibleComponent`) "ECC_Vehicle")
  (`self.SetMats`))

(fn `UserConstructionScript`)