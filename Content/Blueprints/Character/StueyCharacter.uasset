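; Player character with a mark-and-execute revolver ability, plus reload, holstering, HUD and quit-menu handling.
; Holding Aim stops movement and runs a dolly-zoom timeline with post-process and slight time dilation, while clicks mark targets under the cursor decal.
; On release or timeout the timeline reverses, then a delayed ForEach fires at each target, breaking destructibles and spending rounds.
; An alternative top-down camera timeline is present but never runs.
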(event `InputAction|Quit`
  (params (Key :type "Key Structure" :default "AnyKey"))
  (bind _returnvalue (`GameplayStatics.GetPlayerController` 0))
  (bind _quitwidget (`self.QuitWidget`))
  (:`Pressed`
    (`self.SetMovementActive` false :!label _label)
    (`Widget.SetVisibility` _quitwidget "Visible")
    (`WidgetBlueprintLibrary.SetInputMode_UIOnlyEx` _returnvalue _quitwidget)
    (set `PlayerController.bShowMouseCursor` true _returnvalue)))

(event `Key|Q`
  (params (Key :type "Key Structure" :default "AnyKey"))
  (:`Pressed`
    (goto _label)))

(event `InputAction|Reload`
  (params (Key :type "Key Structure" :default "AnyKey"))
  (:`Pressed`
    (`self.Reload`)))

(event `InputAction|DrawWeapon`
  (params (Key :type "Key Structure" :default "AnyKey"))
  (:`Pressed`
    (`self.DrawWeapon` (not (`self.WeaponDrawn`)))))

(event `InputAction|Shoot`
  (params (Key :type "Key Structure" :default "AnyKey"))
  ;[1 1 1] Add Actors to array when clicked - actors in array get shot when top down ends
  (:`Pressed`
    (if (`SceneComponent.IsVisible` (`self.MousePositionDecal`))
      (bind (_hitactor _hitcomponent _hittransform) (`self.GetActorUnderMouse`))
      (`/Engine/EditorBlueprintResources/StandardMacros.IsValid` _hitactor
        (:`Is Valid`
          (bind _location (.location _hittransform))
          (bind _returnvalue (`GameplayStatics.SpawnDecalAttached` "/Game/LowPoly/Stuey/Materials/M_Target_Decal.M_Target_Decal" (16.0 32.0 32.0) _hitcomponent "None" _location (.rotation _hittransform) "KeepWorldPosition"))
          (`KismetArrayLibrary.Array_Add` (`self.PlacedDecals`) _returnvalue)
          (`GameplayStatics.PlaySoundAtLocation` "/Game/SFX/SFX_Cock_Cue.SFX_Cock_Cue" _location))))))

(event `ShootSequence`
  (bind _placeddecals (`self.PlacedDecals`))
  (bind _hitactors (`self.HitActors`))
  ;[1 1 1] Shoot Actors in array
  (if (!= (`KismetArrayLibrary.Array_Length` (`self.HitActors`)) 0)
    (`self.DrawWeapon` true)
    (bind _arrayelement (`self.ForEachWithDelay` _hitactors 0.25)
      (:`LoopBody`
        (set `self.IsAiming` true)
        (`self.AnimNotify_Fire`)
        (for _array_element _placeddecals
          (`/Engine/EditorBlueprintResources/StandardMacros.IsValid` _array_element
            (:`Is Valid`
              (`DecalComponent.SetFadeOut` _array_element 0.0 5.0 false))))
        (`KismetArrayLibrary.Array_Clear` _placeddecals))
      (:`Completed`
        (`KismetArrayLibrary.Array_Clear` _hitactors)
        (set `self.IsAiming` false)))
    (else
      (set `self.IsAiming` false))))

(event `self.AnimNotify_Fire`
  ;[1 1 1] Shoot Actors in array
  (set `self.IsShooting` true)
  (`self.ShootHitActors` (stale `ShootSequence` _arrayelement))
  (`KismetSystemLibrary.Delay` (* (`GameplayStatics.GetWorldDeltaSeconds`) 0.15))
  (set `self.IsShooting` false))

(event `Key|E`
  (params (Key :type "Key Structure" :default "AnyKey"))
  ;[1 1 1] TopDown Aim
)

(event `InputAction|Aim`
  (params (Key :type "Key Structure" :default "AnyKey"))
  ;[1 1 1] DollyZoom
  (:`Pressed`
    (`GameplayStatics.PlaySound2D` "/Engine/EditorSounds/GamePreview/EjectFromPlayer_Cue.EjectFromPlayer_Cue" 2.0 0.85)
    (`self.SetMovementActive` false true)
    (bind (_direction _zoom_fov_stuff) (`Timeline|DollyZoomTimeline` :!label _label_2)
      (:`Update`
        (`self.DollyZoom` _zoom_fov_stuff)
        (bind _returnvalue (`KismetSystemLibrary.K2_SetTimer` self "BulletTimeOver" (`self.BulletTimeMax`)))
        (bind _output_get (set `self.BulletTimeTimer` _returnvalue))
        (set `PostProcessComponent.BlendWeight` _zoom_fov_stuff (`self.PostProcess`))
        (set `self.BulletTimeCurrent` (`KismetSystemLibrary.K2_GetTimerRemainingTimeHandle` _output_get))
        (`GameplayStatics.SetGlobalTimeDilation` (`KismetMathLibrary.Lerp` 1.0 0.95 _zoom_fov_stuff)))
      (:`Finished`
        (if (`|EnumEquality` _direction "Backward")
          (`KismetSystemLibrary.K2_ClearTimer` self "BulletTimeOver")
          (`self.ShootSequence`)))))
  (:`Released`
    (`self.SetMovementActive` true :!label _label_3)
    (goto _label_2 :!via `Reverse`)))

(event `BulletTimeOver`
  ;[1 1 1] DollyZoom
  (goto _label_3))

(event `self.ReceiveTick`
  (params (DeltaSeconds :type "Float (single-precision)"))
  ;[1 1 1] Set Cursor to World Decal Position
  (if (`SceneComponent.IsVisible` (`self.MousePositionDecal`))
    (`self.SetMouseDecalPos`)
    (`self.LookAtCursor`)
    (`self.DrawWeapon` true)))

(event `self.ReceiveBeginPlay`
  (bind _bullettimemax (`self.BulletTimeMax`))
  ;[1 1 1] Begin Play
  (`|ExecutionSequence`
    (:`then_0`
      ;;[1 1 1] Initialise Variables
      (set `self.BulletTimeCurrent` _bullettimemax)
      (bind _returnvalue (`KismetSystemLibrary.K2_SetTimer` null "BulletTimeOver" _bullettimemax))
      (set `self.BulletTimeTimer` _returnvalue)
      (`KismetSystemLibrary.K2_ClearTimer` null "BulletTimeOver"))
    (:`then_1`
      ;;[1 1 1] Setup HUD
      (bind _returnvalue_2 (`|CreateWidget` "/Game/Blueprints/UI/HUD_Master.HUD_Master_C"))
      (bind _output_get (set `self.HUDWidget` _returnvalue_2))
      (`UserWidget.AddToViewport` _output_get 0)
      (bind _returnvalue_3 (`|CreateWidget` "/Game/Blueprints/UI/QuitWidget.QuitWidget_C"))
      (bind _output_get_2 (set `self.QuitWidget` _returnvalue_3))
      (`UserWidget.AddToViewport` _output_get_2 0))))

(fn `DollyZoom`
  (params (FOVAlpha :type "Float (double-precision)"))
  (locals (FOVShort :type "Float (double-precision)" :default 90.0) (FOVLong :type "Float (double-precision)" :default 135.0) (ArmShort :type "Float (double-precision)" :default 430.0) (ArmLong :type "Float (double-precision)" :default 900.0))
  (`CameraComponent.SetFieldOfView` (`self.FollowCamera`) (`KismetMathLibrary.Lerp` (`local.FOVShort`) (`local.FOVLong`) FOVAlpha))
  (set `SpringArmComponent.TargetArmLength` (`KismetMathLibrary.Lerp` (`local.ArmLong`) (`local.ArmShort`) FOVAlpha) (`self.CameraBoom`)))

(fn `DrawWeapon`
  (params (Draw :type Boolean))
  (if Draw
    (`SceneComponent.K2_AttachToComponent` (`self.EquippedWeapon`) (`self.Mesh`) "WeaponSocket" "KeepRelative" "KeepRelative" "KeepRelative" true)
    (set `self.WeaponDrawn` true)
    (else
      (`SceneComponent.K2_AttachToComponent` (`self.EquippedWeapon`) (`self.Mesh`) "Holster" "KeepRelative" "KeepRelative" "KeepRelative" true)
      (set `self.WeaponDrawn` false))))

(fn `GetActorUnderMouse`
  (returns (HitActor :type "Actor Object Reference") (HitComponent :type "PrimitiveComponent Object Reference") (HitTransform :type "Transform Structure"))
  (bind (_bblockinghit _binitialoverlap _time _location _impactpoint _normal _impactnormal _physmat _hitactor _hitcomponent) (`GameplayStatics.BreakHitResult` (`PlayerController.GetHitResultUnderCursorForObjects` (`GameplayStatics.GetPlayerController` 0) (`|MakeArray` "ObjectTypeQuery7" "ObjectTypeQuery6" :!type "EObjectTypeQuery Enum") true)))
  (`/Engine/EditorBlueprintResources/StandardMacros.IsValid` _hitactor
    (:`Is Valid`
      (`KismetArrayLibrary.Array_AddUnique` (`self.HitActors`) _hitactor)
      (return _hitactor _hitcomponent (`KismetMathLibrary.MakeTransform` _location (`KismetMathLibrary.MakeRotationFromAxes` _impactnormal _impactnormal _impactnormal))))
    (:`Is Not Valid`
      (return null null))))

(fn `GetRounds`
  (returns (Rounds :type Integer))
  (return (`self.CurrentRounds`)))

(fn `LookAtCursor`
  (bind _returnvalue (`GameplayStatics.GetPlayerPawn` 0))
  (`self.K2_SetActorRotation` _returnvalue (`KismetMathLibrary.MakeRotator` 0.0 0.0 (.yaw (`KismetMathLibrary.FindLookAtRotation` (`self.K2_GetActorLocation` _returnvalue) (`SceneComponent.K2_GetComponentLocation` (`self.MousePositionDecal`))))) false)
  (set `self.IsAiming` true))

(fn `Reload`
  (if (< (`self.GetRounds`) (`self.MaxRounds`))
    (bind _result (`/Engine/EditorBlueprintResources/StandardMacros.IncrementInt` (`self.CurrentRounds`))
      (:`  `
        (`GameplayStatics.PlaySound2D` "/Game/SFX/revolver_cock.revolver_cock")))))

(fn `SetMouseDecalPos`
  (bind (_bblockinghit _binitialoverlap _time _location _impactpoint _normal _impactnormal) (`GameplayStatics.BreakHitResult` (`PlayerController.GetHitResultUnderCursorByChannel` (`GameplayStatics.GetPlayerController` 0) "TraceTypeQuery1" true)))
  (`SceneComponent.K2_SetWorldLocationAndRotation` (`self.MousePositionDecal`) _location (`KismetMathLibrary.MakeRotationFromAxes` _impactnormal _impactnormal _impactnormal) false false))

(fn `SetMovementActive`
  (params (Active :type Boolean) (ShowMouse :type Boolean))
  (bind _charactermovement (`self.CharacterMovement`))
  (if (not Active)
    (`MovementComponent.StopMovementImmediately` _charactermovement))
  (`ActorComponent.SetActive` _charactermovement Active false)
  (`SceneComponent.SetVisibility` (`self.MousePositionDecal`) ShowMouse false))

(fn `ShootHitActors`
  (params (ActorToShoot :type "Actor Object Reference"))
  (bind _returnvalue (`GameplayStatics.GetPlayerPawn` 0))
  (bind _returnvalue_2 (`self.K2_GetActorLocation` _returnvalue))
  (bind (_returnvalue_location _returnvalue_rotation) (`KismetMathLibrary.BreakTransform` (`SceneComponent.K2_GetComponentToWorld` (`self.Arrow1`))))
  (bind (_returnvalue_roll _returnvalue_pitch _returnvalue_yaw) (`KismetMathLibrary.BreakRotator` (`KismetMathLibrary.FindLookAtRotation` _returnvalue_2 (`self.K2_GetActorLocation` ActorToShoot))))
  (if (> (`self.CurrentRounds`) 0)
    (`/Engine/EditorBlueprintResources/StandardMacros.IsValid` ActorToShoot
      (:`Is Valid`
        (bind _asdestructible_bp (cast `/Game/Blueprints/Props/Destructible_BP` ActorToShoot)
          (:`then`
            (`/Game/Blueprints/Props/Destructible_BP.BreakMe` _asdestructible_bp))
          (:`CastFailed`
            (`KismetSystemLibrary.PrintString` (`KismetSystemLibrary.GetDisplayName` ActorToShoot))))
        (`self.K2_SetActorRotation` _returnvalue (`KismetMathLibrary.MakeRotator` 0.0 0.0 _returnvalue_yaw) false)
        (`|SpawnActorFromClass` "/Game/Blueprints/Character/BP_Projectile.BP_Projectile_C" (`KismetMathLibrary.MakeTransform` _returnvalue_location _returnvalue_rotation) "AlwaysSpawn" "OverrideRootScale")
        (`GameplayStatics.PlaySoundAtLocation` "/Game/SFX/SFX_Revolver_Shot_Cue.SFX_Revolver_Shot_Cue" _returnvalue_2)
        (bind _result (`/Engine/EditorBlueprintResources/StandardMacros.DecrementInt` (`self.CurrentRounds`))
          (:`  `
            (`GameplayStatics.PlayWorldCameraShake` "/Game/Blueprints/Character/CamShake_01.CamShake_01_C" (`self.K2_GetActorLocation` (`GameplayStatics.GetPlayerPawn` 0)) 0.0 1000.0)))))
    (else
      (`KismetArrayLibrary.Array_Clear` (`self.HitActors`))
      (`GameplayStatics.PlaySoundAtLocation` "/Game/StarterContent/Audio/Explosion01.Explosion01")
      (`KismetSystemLibrary.PrintString` "ClipEmpty"))))

(fn `TopDownRotation`
  (params (RotationAlpha :type "Float (double-precision)"))
  (locals (EndRotation :type "Rotator Structure" :default (struct :`Pitch` -90.0)) (StartRotation :type "Rotator Structure" :default (struct :`Pitch` -30.0)))
  (`SceneComponent.K2_SetRelativeRotation` (`self.CameraBoom`) (`KismetMathLibrary.RLerp` (`local.StartRotation`) (`local.EndRotation`) RotationAlpha) false false))

(fn `UserConstructionScript`)