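; InputManager is a Blueprint that tracks whether the player's latest action input came from a gamepad.
; Pressed events for menu-style and combat input actions each pass their key to CheckInputType and store the result in GamepadActive.
; CheckInputType counts gamepad keys and any float-axis key as gamepad input.
; Both the key name and the resulting flag are printed for debugging.
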(event `InputAction|DrawWeapon` :consume false :overrideparent false
  (params (Key :type "Key Structure" :default "AnyKey"))
  (:`Pressed`
    (bind _isgamepad (`self.CheckInputType` Key)
      (:`Out`
        (set `self.GamepadActive` _isgamepad)
        (`KismetSystemLibrary.PrintString` (`KismetStringLibrary.Conv_BoolToString` (`self.GamepadActive`)) :!label _label)))))

(event `InputAction|Quit` :consume false :overrideparent false
  (params (Key :type "Key Structure" :default "AnyKey"))
  (:`Pressed`
    (bind _isgamepad (`self.CheckInputType` Key)
      (:`Out`
        (set `self.GamepadActive` _isgamepad)
        (goto _label)))))

(event `InputAction|Aim` :consume false :overrideparent false
  (params (Key :type "Key Structure" :default "AnyKey"))
  (:`Pressed`
    (bind _isgamepad (`self.CheckInputType` Key)
      (:`Out`
        (set `self.GamepadActive` _isgamepad)
        (goto _label)))))

(event `InputAction|Shoot` :consume false :overrideparent false
  (params (Key :type "Key Structure" :default "AnyKey"))
  (:`Pressed`
    (bind _isgamepad (`self.CheckInputType` Key)
      (:`Out`
        (set `self.GamepadActive` _isgamepad)
        (goto _label)))))

(event `InputAction|Reload` :consume false :overrideparent false
  (params (Key :type "Key Structure" :default "AnyKey"))
  (:`Pressed`
    (bind _isgamepad (`self.CheckInputType` Key)
      (:`Out`
        (set `self.GamepadActive` _isgamepad)
        (goto _label)))))

(event `InputAction|Confirm` :consume false :overrideparent false
  (params (Key :type "Key Structure" :default "AnyKey"))
  (:`Pressed`
    (bind _isgamepad (`self.CheckInputType` Key)
      (:`Out`
        (set `self.GamepadActive` _isgamepad)
        (goto _label)))))

(event `InputAction|Down` :consume false :overrideparent false
  (params (Key :type "Key Structure" :default "AnyKey"))
  (:`Pressed`
    (bind _isgamepad (`self.CheckInputType` Key)
      (:`Out`
        (set `self.GamepadActive` _isgamepad)
        (goto _label)))))

(event `InputAction|Right` :consume false :overrideparent false
  (params (Key :type "Key Structure" :default "AnyKey"))
  (:`Pressed`
    (bind _isgamepad (`self.CheckInputType` Key)
      (:`Out`
        (set `self.GamepadActive` _isgamepad)
        (goto _label)))))

(event `InputAction|Left` :consume false :overrideparent false
  (params (Key :type "Key Structure" :default "AnyKey"))
  (:`Pressed`
    (bind _isgamepad (`self.CheckInputType` Key)
      (:`Out`
        (set `self.GamepadActive` _isgamepad)
        (goto _label)))))

(event `InputAction|Up` :consume false :overrideparent false
  (params (Key :type "Key Structure" :default "AnyKey"))
  (:`Pressed`
    (bind _isgamepad (`self.CheckInputType` Key)
      (:`Out`
        (set `self.GamepadActive` _isgamepad)
        (goto _label)))))

(fn `UserConstructionScript`)