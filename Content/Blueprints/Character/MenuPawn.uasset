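; MenuPawn is the pawn for the front-end menu, handling navigation between splash screen, main menu, new game and quit prompt.
; On BeginPlay it starts music through the AudioManager and initialises the HUD_BP.
; Confirm, Quit, Reload and Backspace inputs switch on EMenuState, calling transition functions that drive HUD widgets, swap tracks and set focus.
; Inputs also detect gamepad use, so Tick hides the mouse cursor for gamepad players.
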(event `self.ReceiveTick`
  (params (DeltaSeconds :type "Float (single-precision)"))
  (set `PlayerController.bShowMouseCursor` (not (`self.IsGamepad`)) (`GameplayStatics.GetPlayerController` 0)))

(event `self.ReceiveBeginPlay`
  (`|ExecutionSequence`
    (:`then_0`
      (bind _outactors (`GameplayStatics.GetAllActorsOfClass` "/Game/Blueprints/Game/AudioManager.AudioManager_C"))
      (bind _item (`KismetArrayLibrary.Array_Get` _outactors))
      (bind _output_get (set `self.AudioManager` _item))
      (`/Game/Blueprints/Game/AudioManager.StartMusic` _item (`self.StartMusic`))
      (`/Game/Blueprints/Game/AudioManager.StartMusic` _output_get (`self.StartMusic`)))
    (:`then_1`
      (bind _ashud_bp (cast `/Game/Blueprints/Game/HUD_BP` (`PlayerController.GetHUD` (`GameplayStatics.GetPlayerController` 0))))
      (bind _output_get_2 (set `self.MyHUD` _ashud_bp))
      (`/Game/Blueprints/UI/WidgetBasedMacros.SetInMenu` true
        (:`Out`
          (`/Game/Blueprints/Game/HUD_BP.InitialiseHUD` _output_get_2))))))

(event `InputAction|Quit` :consume false :overrideparent false
  (params (Key :type "Key Structure" :default "AnyKey"))
  (:`Pressed`
    (`/Game/Blueprints/UI/WidgetBasedMacros.IsGamepad` Key
      (:`True`
        (set `self.IsGamepad` true))
      (:`False`
        (set `self.IsGamepad` false)))
    (`/Game/Blueprints/UI/WidgetBasedMacros.IsInMenu`
      (:`True`
        (switch `/Game/Blueprints/UI/Menus/EMenuState` (`self.EMenuState`)
          (:`NewEnumerator0`
            (`/Game/Blueprints/UI/Menus/QuitWidget.ShowQuit` (`/Game/Blueprints/Game/HUD_BP.QuitWidget` (`self.MyHUD`))))
          (:`NewEnumerator1`
            (`self.MenuToSplash`))
          (:`NewEnumerator2`
            (`self.NewGameToMenu`))
          (:`NewEnumerator5`
            (`self.QuitToMenu`)))))))

(event `InputAction|Confirm`
  (params (Key :type "Key Structure" :default "AnyKey"))
  (:`Pressed`
    (`self.CheckGamepad` Key
      (:`Out`
        (switch `/Game/Blueprints/UI/Menus/EMenuState` (`self.EMenuState`)
          (:`NewEnumerator0`
            (`self.SplashToMenu`))
          (:`NewEnumerator2`
            (`/Game/Blueprints/UI/Menus/MainMenuWidget.CommitTextBox` (`/Game/Blueprints/Game/HUD_BP.MainMenuWidget` (`self.MyHUD`)) "" "OnEnter"))
          (:`NewEnumerator5`
            (`KismetSystemLibrary.QuitGame` null "Quit")))))))

(event `InputAction|Reload`
  (params (Key :type "Key Structure" :default "AnyKey"))
  (:`Pressed`
    (`/Game/Blueprints/UI/WidgetBasedMacros.IsGamepad` Key
      (:`True`
        (set `self.IsGamepad` true))
      (:`False`
        (set `self.IsGamepad` false :!label _label)))
    (switch `/Game/Blueprints/UI/Menus/EMenuState` (`self.EMenuState`)
      (:`NewEnumerator0`
        (`/Game/Blueprints/UI/Menus/QuitWidget.ShowQuit` (`/Game/Blueprints/Game/HUD_BP.QuitWidget` (`self.MyHUD`))))
      (:`NewEnumerator1`
        (`self.MenuToSplash`))
      (:`NewEnumerator2`
        (`self.NewGameToMenu`))
      (:`NewEnumerator5`
        (`self.QuitToMenu`)))))

(event `Key|BackSpace`
  (params (Key :type "Key Structure" :default "AnyKey"))
  (:`Pressed`
    (goto _label)))

(fn `MenuToSplash`
  (bind _mainmenuwidget (`/Game/Blueprints/Game/HUD_BP.MainMenuWidget` (`self.MyHUD`)))
  (`/Game/Blueprints/UI/Menus/MainMenuWidget.MenuToSplashTransition` _mainmenuwidget)
  (`/Game/Blueprints/Game/AudioManager.ChangeTrack` (`self.AudioManager`) "/Game/SFX/Music/BGMusic_Cue.BGMusic_Cue" 2.0)
  (`self.SetShowCursor` _mainmenuwidget
    (:`Out`
      (set `self.EMenuState` "NewEnumerator0"))))

(fn `NewGameToMenu`
  (bind _mainmenuwidget (`/Game/Blueprints/Game/HUD_BP.MainMenuWidget` (`self.MyHUD`)))
  (`/Game/Blueprints/UI/Menus/MainMenuWidget.ResetNewGame` _mainmenuwidget)
  (`self.SetShowCursor` (`PanelWidget.GetChildAt` (`/Game/Blueprints/UI/Menus/MainMenuWidget.VerticalBox` _mainmenuwidget) 0)))

(fn `QuitToMenu`
  (bind _myhud (`self.MyHUD`))
  (`/Game/Blueprints/UI/Menus/QuitWidget.HideQuit` (`/Game/Blueprints/Game/HUD_BP.QuitWidget` _myhud))
  (`self.SetWidgetInFocus` (`/Game/Blueprints/UI/Menus/MainMenuWidget.TitleScreen` (`/Game/Blueprints/Game/HUD_BP.MainMenuWidget` _myhud)))
  (set `self.EMenuState` "NewEnumerator0"))

(fn `SetWidgetInFocus`
  (params (InWidgetToFocus :type "Widget Object Reference"))
  (`self.SetShowCursor` InWidgetToFocus))

(fn `SplashToMenu`
  (bind _mainmenuwidget (`/Game/Blueprints/Game/HUD_BP.MainMenuWidget` (`self.MyHUD`)))
  (`GameplayStatics.PlaySound2D` "/Game/SFX/Effects/StartGameGunShot_Cue.StartGameGunShot_Cue" 0.75)
  (`/Game/Blueprints/Game/AudioManager.ChangeTrack` (`self.AudioManager`) "/Game/SFX/Music/GoodBad_Cue.GoodBad_Cue" 0.0)
  (`/Game/Blueprints/UI/Menus/MainMenuWidget.SplashToMenuTransition` _mainmenuwidget)
  (`self.SetShowCursor` (`PanelWidget.GetChildAt` (`/Game/Blueprints/UI/Menus/MainMenuWidget.VerticalBox` _mainmenuwidget) 0)
    (:`Out`
      (set `self.EMenuState` "NewEnumerator1"))))

(fn `UserConstructionScript`)